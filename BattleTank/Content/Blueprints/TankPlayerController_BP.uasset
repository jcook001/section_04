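; Player controller Blueprint for a tank game that manages the player's HUD and a pausing debug menu.
; BeginPlay creates both widgets but adds only the player UI, stored as Crosshair, to the viewport.
; Releasing Show Debug toggles the menu, pause state and input mode, while Tick syncs the mouse cursor to menu visibility.
; The node passing the tank's aiming component to the player UI is disconnected and never runs.
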(event EventBeginPlay
  (bind _returnvalue (Game|GetPlayerController 0))
  (bind _returnvalue_2 (UserInterface|CreateWidget "/Game/UI/DebugMenu_BP.DebugMenu_BP_C" _returnvalue))
  (Variables|Default|SetDebug%20Menu _returnvalue_2)
  (bind _returnvalue_3 (UserInterface|CreateWidget "/Game/UI/PlayerUI_BP.PlayerUI_BP_C" _returnvalue))
  (bind _output_get (Variables|Default|SetCrosshair _returnvalue_3))
  (UserInterface|Viewport|AddtoViewport _output_get 0))

(event EventTick
  (params (DeltaSeconds :type Float%20%28single-precision%29))
  ;[1 1 1] Always show mouse with debug menu on screen
  (Variables|Default|SetbShowMouseCursor (UserInterface|Viewport|IsinViewport (Variables|Default|GetDebug%20Menu))))

(event Input|ActionEvents|InputActionShowDebug
  (params (Key :type Key%20Structure :default "None"))
  (bind _returnvalue (Game|GetPlayerController 0))
  (bind _debug_menu (Variables|Default|GetDebug%20Menu))
  (:Released
    (switch int (Math|Conversions|ToInteger(Boolean) (UserInterface|Viewport|IsinViewport (Variables|Default|GetDebug%20Menu)))
      (:0
        (Game|SetGamePaused true)
        (UserInterface|Viewport|AddtoViewport _debug_menu 0)
        (Input|SetInputModeGameandUI _returnvalue _debug_menu "DoNotLock" false))
      (:1
        (Game|SetGamePaused false)
        (Widget|RemovefromParent _debug_menu)
        (Input|SetInputModeGameOnly _returnvalue)))))

(fn ConstructionScript)